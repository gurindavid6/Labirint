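; BP_Door is a door that consumes one of the player's keys when interacted with and plays an opening animation.
; Interact checks BP_Player's NumberOfKeys, decrements it, then adds a static mesh component, stores it as KeyHole and calls attach with KeyHole as its own parent.
; The DoorOpening timeline then drives KeyMesh along relative Y and DoorMesh along relative Z.
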(event `/Game/Blueprint/BPI/BPI_Interaction.Interact`
  (params (Actor :type "Actor Object Reference"))
  (`/Engine/EditorBlueprintResources/StandardMacros.IsValid` (`self.DoorMesh`)
    (:`Is Valid`
      (bind _asbp_player (cast `/Game/PLAYER/BP_Player` (`GameplayStatics.GetPlayerCharacter` 0)))
      (bind _numberofkeys (`/Game/PLAYER/BP_Player.NumberOfKeys` _asbp_player))
      (if (> _numberofkeys 0)
        (`/Engine/EditorBlueprintResources/StandardMacros.DecrementInt` _numberofkeys
          (:`  `
            (bind _returnvalue (`AddComponent|NODE_AddStaticMeshComponent-0`))
            (bind _output_get (set `self.KeyHole` _returnvalue))
            (`SceneComponent.K2_AttachToComponent` _output_get (`self.KeyHole`) "None" "SnapToTarget" "SnapToTarget" "SnapToTarget" true)
            (bind (_direction _keyposition _doorposition) (`Timeline|DoorOpening` :!via `PlayFromStart`)
              (:`Update`
                (`SceneComponent.K2_SetRelativeLocation` (`self.KeyMesh`) (`KismetMathLibrary.MakeVector` 0.0 _keyposition) false false)
                (`SceneComponent.K2_SetRelativeLocation` (`self.DoorMesh`) (`KismetMathLibrary.MakeVector` 0.0 0.0 _doorposition) false false)))))))))

(fn `UserConstructionScript`)