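; BP_Shoot is an arrow-shooter trap that fires BP_Arrow from its Arrow component when the player steps into its line of fire.
; Tick sphere-traces a short distance forward on the Camera channel and fires if it hits a living BP_Player.
; A DoOnce reset after a short delay throttles shots.
; A long looping timer also triggers firing regardless of the trace, and is cleared if the shoot event finds the player dead.
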(event `self.ReceiveBeginPlay`
  (`self.GetPlayer Ref`)
  (bind _returnvalue (`KismetSystemLibrary.K2_SetTimerDelegate` (delegate `ShoorArrow`) 500.0 true))
  (set `self.TimerHandle` _returnvalue))

(event `ShoorArrow`
  (`/Engine/EditorBlueprintResources/StandardMacros.IsValid` (`self.As BP Player`)
    (:`Is Valid`
      (if (`/Game/PLAYER/BP_Player.PlayerisDead` (`self.As BP Player`))
        (`KismetSystemLibrary.K2_ClearAndInvalidateTimerHandle` (`self.TimerHandle`))
        (else
          (`/Engine/EditorBlueprintResources/StandardMacros.DoOnce` false :!label _label
            (:`Completed`
              (`self.Arrow Spawn`)
              (`KismetSystemLibrary.Delay` 0.5)
              (goto _label :!via `Reset`))))))))

(event `self.ReceiveTick`
  (params (DeltaSeconds :type "Float (single-precision)"))
  (bind _arrow (`self.Arrow`))
  (bind _as_bp_player (`self.As BP Player`))
  (bind _returnvalue (`SceneComponent.K2_GetComponentLocation` _arrow))
  (bind _outhit (`KismetSystemLibrary.SphereTraceSingle` :`Start` _returnvalue :`End` (+ _returnvalue (* (`KismetMathLibrary.GetForwardVector` (`SceneComponent.K2_GetComponentRotation` _arrow)) 250)) :`Radius` 10.0 :`TraceChannel` "TraceTypeQuery2" :`DrawTime` 20.0))
  (`/Engine/EditorBlueprintResources/StandardMacros.IsValid` (`self.As BP Player`)
    (:`Is Valid`
      (if (and (== (`.HitActor` (`GameplayStatics.BreakHitResult` _outhit)) _as_bp_player) (not (`/Game/PLAYER/BP_Player.PlayerisDead` _as_bp_player)))
        (`self.ShoorArrow`)))))

(fn `Arrow Spawn`
  (`|SpawnActorFromClass` "/Game/Blueprint/BP_Arrow.BP_Arrow_C" (`SceneComponent.K2_GetComponentToWorld` (`self.Arrow`)) "Undefined" "MultiplyWithRoot" null null))

(fn `GetPlayer Ref`
  (bind _asbp_player (cast `/Game/PLAYER/BP_Player` (`GameplayStatics.GetPlayerCharacter` 0)))
  (set `self.As BP Player` _asbp_player))

(fn `UserConstructionScript`)