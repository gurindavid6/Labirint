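; BP_Arrow is an arrow actor that damages and knocks back the player on impact.
; Its Sphere hit event calls DestroyActor first on any hit, then continues only if the hit actor is a BP_Player with Health above zero.
; That player is launched by the arrow's velocity plus an upward boost and takes fixed damage, followed by a second DestroyActor call.
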(event `self.Sphere.OnComponentHit`
  (params (HitComponent :type "PrimitiveComponent Object Reference") (OtherActor :type "Actor Object Reference") (OtherComp :type "PrimitiveComponent Object Reference") (NormalImpulse :type "Vector Structure") (Hit :type "HitResult Structure (by ref)"))
  (`self.K2_DestroyActor`)
  (bind _asbp_player (cast `/Game/PLAYER/BP_Player` OtherActor))
  (set `self.As BP Player` _asbp_player)
  (if (> (`/Game/PLAYER/BP_Player.Health` _asbp_player) 0)
    (`Character.LaunchCharacter` _asbp_player (+ (`self.GetVelocity`) (0.0 0.0 200.0)) false false)
    (`GameplayStatics.ApplyDamage` (`self.As BP Player`) 1.0)
    (`self.K2_DestroyActor`)))

(fn `UserConstructionScript`)